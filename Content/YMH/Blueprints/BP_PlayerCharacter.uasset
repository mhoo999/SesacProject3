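; BP_PlayerCharacter is a player character Blueprint that serves as a debug driver for the enemy dummy BP_EnemyDummy_OSH.
; BeginPlay finds the dummy with GetActorOfClass and caches the reference.
; Debug key events on Q, W, E and R call its attack, defence, release and hand-rotation functions directly, with no validity check.
; Tick and overlap events are unused, and the construction script is empty.
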(event EventBeginPlay
  (bind _returnvalue (Actor|GetActorOfClass "/Game/OSH/Blueprint/Character/BP_EnemyDummy_OSH.BP_EnemyDummy_OSH_C"))
  (Variables|Default|SetDummy _returnvalue))

(event Collision|EventActorBeginOverlap
  (params (OtherActor :type Actor%20Object%20Reference)))

(event EventTick
  (params (DeltaSeconds :type Float%20%28single-precision%29)))

(event Input|KeyboardEvents|DebugKeyE
  (params (Key :type Key%20Structure :default "None") (ActionValue :type Input%20Action%20Value%20Structure))
  (:Pressed
    (Class|EnemyBase|Release (Variables|Default|GetDummy))))

(event Input|KeyboardEvents|DebugKeyQ
  (params (Key :type Key%20Structure :default "None") (ActionValue :type Input%20Action%20Value%20Structure))
  (:Pressed
    (Class|EnemyBase|Attack (Variables|Default|GetDummy))))

(event Input|KeyboardEvents|DebugKeyW
  (params (Key :type Key%20Structure :default "None") (ActionValue :type Input%20Action%20Value%20Structure))
  (:Pressed
    (Class|EnemyBase|Defence (Variables|Default|GetDummy))))

(event Input|KeyboardEvents|DebugKeyR
  (params (Key :type Key%20Structure :default "None") (ActionValue :type Input%20Action%20Value%20Structure))
  (:Pressed
    (Class|EnemyDummy|AddHandRotaiton (Variables|Default|GetDummy))))

(fn ConstructionScript)