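; Player character child Blueprint that equips the player with a weapon when play begins.
; After the parent BeginPlay, it spawns a BP_WeaponBase actor, stores it as Weapon and attaches it to RightHandMesh.
; It then applies a fixed relative offset and rotation and registers itself as the weapon's owning player.
; Tick, overlap and construction add no logic of their own.
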(event `self.ReceiveBeginPlay`
  (bind _weapon (`self.Weapon`))
  (`parent.ReceiveBeginPlay`)
  (bind _returnvalue (`|SpawnActorFromClass` "/Game/OSH/Blueprint/Weapon/BP_WeaponBase.BP_WeaponBase_C" (`KismetMathLibrary.MakeTransform` (0.0 0.0 0.0)) "Undefined" "MultiplyWithRoot" null null))
  (bind _output_get (set `self.Weapon` _returnvalue))
  (`self.K2_AttachToComponent` _output_get (`self.RightHandMesh`) "None" "KeepRelative" "KeepRelative" "KeepRelative" true)
  (`self.K2_SetActorRelativeLocation` _weapon (40.0 21.0 -3.0) false false)
  (`self.K2_SetActorRelativeRotation` _weapon (struct :`Yaw` 20.0) false false)
  (`WeaponBase.SetOwningPlayer` _weapon self))

(fn `UserConstructionScript`
  (`parent.UserConstructionScript`))