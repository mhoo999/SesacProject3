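; Player character child Blueprint that equips a weapon and adds debug shortcuts for the main menu.
; On BeginPlay it runs the parent logic, spawns a BP_WeaponBase, attaches it to RightHandMesh with a fixed offset and registers itself as the owning player.
; Debug keys H, J and K reach the MainMenuWidget through BP_MainMenuGameMode's widget actor to trigger single play, multiplayer and join game.
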(event EventBeginPlay
  (|CallParentFunction)
  (bind _returnvalue (Game|SpawnActorfromClass "/Game/OSH/Blueprint/Weapon/BP_WeaponBase.BP_WeaponBase_C" (Math|Transform|MakeTransform "0, 0, 0" "0, 0, 0" "1.000000,1.000000,1.000000") "Undefined" "MultiplyWithRoot" 0 0))
  (bind _output_get (Variables|Default|SetWeapon _returnvalue))
  (Transformation|AttachComponentToComponent _output_get (Variables|Default|GetRightHandMesh) "None" "KeepRelative" "KeepRelative" "KeepRelative" true)
  (Transformation|SetActorRelativeLocation (Variables|Default|GetWeapon) "40.000000,21.000000,-3.000000")
  (Transformation|SetActorRelativeRotation (Variables|Default|GetWeapon) "0.000000,20.000000,0.000000")
  (Class|WeaponBase|SetOwningPlayer (Variables|Default|GetWeapon) self))

(event Collision|EventActorBeginOverlap
  (params (OtherActor :type Actor%20Object%20Reference))
  (|CallParentFunction OtherActor) ; This node is disabled and will not be called.\nDrag off pins to build functionality.
)

(event EventTick
  (params (DeltaSeconds :type Float%20%28single-precision%29))
  (|CallParentFunction DeltaSeconds) ; This node is disabled and will not be called.\nDrag off pins to build functionality.
)

(event Input|KeyboardEvents|DebugKeyK
  (params (Key :type Key%20Structure) (ActionValue :type Input%20Action%20Value%20Structure))
  (:Pressed
    (bind _asbp_main_menu_game_mode (Utilities|Casting|CastToBP_MainMenuGameMode (Game|GetGameMode)))
    (bind _asmain_menu_widget (Utilities|Casting|CastToMainMenuWidget (UserInterface|GetWidget (Variables|/Game/OSH/Blueprint/Actor/BP_MainMenuWidgetActor.BP_MainMenuWidgetActor_C|GetWidget (Variables|/Game/OSH/Blueprint/GameMode/BP_MainMenuGameMode.BP_MainMenuGameMode_C|GetMainMenuWidgetActor _asbp_main_menu_game_mode)))))
    (Class|MainMenuWidget|PresJoinGame _asmain_menu_widget)))

(event Input|KeyboardEvents|DebugKeyH
  (params (Key :type Key%20Structure) (ActionValue :type Input%20Action%20Value%20Structure))
  (:Pressed
    (bind _asbp_main_menu_game_mode (Utilities|Casting|CastToBP_MainMenuGameMode (Game|GetGameMode)))
    (bind _asmain_menu_widget (Utilities|Casting|CastToMainMenuWidget (UserInterface|GetWidget (Variables|/Game/OSH/Blueprint/Actor/BP_MainMenuWidgetActor.BP_MainMenuWidgetActor_C|GetWidget (Variables|/Game/OSH/Blueprint/GameMode/BP_MainMenuGameMode.BP_MainMenuGameMode_C|GetMainMenuWidgetActor _asbp_main_menu_game_mode)))))
    (Class|MainMenuWidget|PressSinglePlay _asmain_menu_widget)))

(event Input|KeyboardEvents|DebugKeyJ
  (params (Key :type Key%20Structure) (ActionValue :type Input%20Action%20Value%20Structure))
  (:Pressed
    (bind _asbp_main_menu_game_mode (Utilities|Casting|CastToBP_MainMenuGameMode (Game|GetGameMode)))
    (bind _asmain_menu_widget (Utilities|Casting|CastToMainMenuWidget (UserInterface|GetWidget (Variables|/Game/OSH/Blueprint/Actor/BP_MainMenuWidgetActor.BP_MainMenuWidgetActor_C|GetWidget (Variables|/Game/OSH/Blueprint/GameMode/BP_MainMenuGameMode.BP_MainMenuGameMode_C|GetMainMenuWidgetActor _asbp_main_menu_game_mode)))))
    (Class|MainMenuWidget|PressMultiPlay _asmain_menu_widget)))

(fn ConstructionScript
  (|CallParentFunction))